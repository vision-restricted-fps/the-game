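; Melee enemy Blueprint that roams, chases the player on sight and dies when a bullet hits it.
; Pawn sensing sets a one-second sight flag that switches recursive AI move events between slow random roaming and a faster chase, rechecked on a delay.
; Within chase radius, ShootPlayer turns it toward the player, stops it and plays an animation, without spawning projectiles or resuming the loop.
; Bullet overlap on Mortality updates the player's enemy count and destroys it.
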(event OnSeePawn(PawnSensing)
  (params (Pawn :type Pawn%20Object%20Reference))
  ;[0.1899 1 0.2222] On See Pawn
  (Variables|Default|SetseesPlayer true)
  (Utilities|FlowControl|Delay 1.0)
  (Variables|Default|SetseesPlayer false))

(event OnComponentBeginOverlap(mortality)
  (params (OverlappedComponent :type Primitive%20Component%20Object%20Reference) (OtherActor :type Actor%20Object%20Reference) (OtherComp :type Primitive%20Component%20Object%20Reference) (OtherBodyIndex :type Integer) (bFromSweep :type Boolean) (SweepResult :type Hit%20Result%20Structure%20%28by%20ref%29))
  (Utilities|Casting|CastToBP_Bullet OtherActor)
  (bind _asbp_first_person_character (Utilities|Casting|CastToBP_FirstPersonCharacter (Game|Player|GetPlayerPawn 0)))
  (Default|EventUpdateEnemyCnt _asbp_first_person_character)
  (Actor|DestroyActor))

(event Custom|Chase%20Player
  ;[0.553 0.3394 1] Chase Player
  (if (Variables|Default|GetseesPlayer)
    (if (<= (Transformation|GetDistanceTo (Game|GetPlayerCharacter 0) self) (Variables|Default|GetChaseRadius))
      (CallFunction|ShootPlayer)
      (else
        (Rendering|SetVisibility (Variables|Default|GetSK_EnemyRifle) false false)
        (Variables|/Script/Engine.CharacterMovementComponent|SetMaxWalkSpeed (Variables|Character|GetCharacterMovement) 6e+02)
        (AI|AIMoveTo self "0, 0, 0" (Game|GetPlayerCharacter 0) 5.0 false
          (:then
            (Utilities|FlowControl|Delay 1.0)
            (CallFunction|ChasePlayer)))))
    (else
      (Rendering|SetVisibility (Variables|Default|GetSK_EnemyRifle) false false)
      (CallFunction|Roam))))

(event Custom|Roam
  ;[1 0.9434 0.4534] Roam
  (if (Variables|Default|GetseesPlayer)
    (CallFunction|ChasePlayer)
    (else
      (Variables|/Script/Engine.CharacterMovementComponent|SetMaxWalkSpeed (Variables|Character|GetCharacterMovement) 2e+02)
      (AI|AIMoveTo self (.RandomLocation (AI|Navigation|GetRandomReachablePointinRadius (Transformation|GetActorLocation) 3e+02 0 0)) 0 5.0 false
        (:OnSuccess
          _)
        (:OnFail
          _))
      (CallFunction|Roam))))

(event Custom|Shoot%20Player
  ;[1 0.3212 0.3212] Shoot Player
  (Transformation|SetActorRotation (Math|Rotator|FindLookatRotation (Transformation|GetWorldLocation (Variables|Default|GetProjectileSpawn)) (Transformation|GetActorLocation (Game|GetPlayerCharacter 0))))
  (Variables|/Script/Engine.CharacterMovementComponent|SetMaxWalkSpeed (Variables|Character|GetCharacterMovement) 0.0)
  (Components|Animation|PlayAnimation (Variables|Character|GetMesh) 0 false))

(event EventBeginPlay
  ;[0.45 1 0.5922] Begin Play
  (CallFunction|Roam))

(event EventTick
  (params (DeltaSeconds :type Float%20%28single-precision%29)))

(fn ConstructionScript)

(fn Death
  (Actor|DestroyActor))